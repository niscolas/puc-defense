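; BP_PlayerNew is the player Blueprint for a game that combines weapon firing with tower placement.
; On BeginPlay it sets the camera as the placement line-trace origin and Arrow1 as the weapon spawn point, then spawns weapons.
; Enhanced Input actions, gated by IsInputEnabled, forward to movement, look, firing, three-slot tower selection and placement functions, whose logic lives outside these graphs.
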(event Input|EnhancedActionEvents|EnhancedInputActionIA_Move
  (params (ActionValue :type Vector%202D%20Structure) (ElapsedSeconds :type Float%20%28double-precision%29) (TriggeredSeconds :type Float%20%28double-precision%29) (InputAction :type Input%20Action%20Object%20Reference :default "/Game/_MainContent/Player/IA_Move.IA_Move"))
  (if (Variables|Default|GetIsInputEnabled)
    (Class|DefaultPlayer|Move ActionValue)))

(event Input|EnhancedActionEvents|EnhancedInputActionIA_Look
  (params (ActionValue :type Vector%202D%20Structure) (ElapsedSeconds :type Float%20%28double-precision%29) (TriggeredSeconds :type Float%20%28double-precision%29) (InputAction :type Input%20Action%20Object%20Reference :default "/Game/_MainContent/Player/IA_Look.IA_Look"))
  (if (Variables|Default|GetIsInputEnabled)
    (Class|DefaultPlayer|Look ActionValue)))

(event Input|EnhancedActionEvents|EnhancedInputActionIA_PlaceTower
  (params (ActionValue :type Boolean) (ElapsedSeconds :type Float%20%28double-precision%29) (TriggeredSeconds :type Float%20%28double-precision%29) (InputAction :type Input%20Action%20Object%20Reference :default "/Game/_MainContent/Player/IA_PlaceTower.IA_PlaceTower"))
  (:Started
    (if (and ActionValue (Variables|Default|GetIsInputEnabled))
      (Class|DefaultPlayer|PlaceTower))))

(event Input|EnhancedActionEvents|EnhancedInputActionIA_Fire
  (params (ActionValue :type Boolean) (ElapsedSeconds :type Float%20%28double-precision%29) (TriggeredSeconds :type Float%20%28double-precision%29) (InputAction :type Input%20Action%20Object%20Reference :default "/Game/_MainContent/Player/IA_Fire.IA_Fire"))
  (:Started
    (if (Variables|Default|GetIsInputEnabled)
      (Class|DefaultPlayer|FireWeapon))))

(event Input|EnhancedActionEvents|EnhancedInputActionIA_SelectTower1
  (params (ActionValue :type Boolean) (ElapsedSeconds :type Float%20%28double-precision%29) (TriggeredSeconds :type Float%20%28double-precision%29) (InputAction :type Input%20Action%20Object%20Reference :default "/Game/_MainContent/Player/IA_SelectTower1.IA_SelectTower1"))
  (:Started
    (if (and ActionValue (Variables|Default|GetIsInputEnabled))
      (Class|DefaultPlayer|SelectTower))))

(event Input|EnhancedActionEvents|EnhancedInputActionIA_SelectTower2
  (params (ActionValue :type Boolean) (ElapsedSeconds :type Float%20%28double-precision%29) (TriggeredSeconds :type Float%20%28double-precision%29) (InputAction :type Input%20Action%20Object%20Reference :default "/Game/_MainContent/Player/IA_SelectTower2.IA_SelectTower2"))
  (:Started
    (if (and ActionValue (Variables|Default|GetIsInputEnabled))
      (Class|DefaultPlayer|SelectTower 1))))

(event Input|EnhancedActionEvents|EnhancedInputActionIA_SelectTower3
  (params (ActionValue :type Boolean) (ElapsedSeconds :type Float%20%28double-precision%29) (TriggeredSeconds :type Float%20%28double-precision%29) (InputAction :type Input%20Action%20Object%20Reference :default "/Game/_MainContent/Player/IA_SelectTower3.IA_SelectTower3"))
  (:Started
    (if (and ActionValue (Variables|Default|GetIsInputEnabled))
      (Class|DefaultPlayer|SelectTower 2))))

(event EventBeginPlay
  (Variables|Default|SetPlacementLineTraceOrigin (Variables|Default|GetCamera))
  (Variables|Default|SetWeaponsSpawnPoint (Variables|Default|GetArrow1))
  (Class|DefaultPlayer|SpawnWeapons))

(fn ConstructionScript)